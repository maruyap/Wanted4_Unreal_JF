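; BP_Player2 is the second player's fighter character, registering itself with BP_GameMode as RefPlayer2 on BeginPlay.
; Remote_ input events drive movement, jump, guard and attack, gated by CanPerformAction, guard and StateBP checks.
; A quick repeated move input starts a dash, whose attack launches the character with input locked and friction removed.
; Normal attacks play a three-punch montage, queuing NextCombo from the current section.
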(event `self.ReceiveBeginPlay`
  (`parent.ReceiveBeginPlay`)
  (bind _asbp_game_mode (cast `/Game/BluePrints/Character/BP_GameMode` (`GameplayStatics.GetGameMode`)))
  (set `/Game/BluePrints/Character/BP_GameMode.Ref_Player2` self _asbp_game_mode))

(event `Remote_Jump_Started`
  ;[0.00526 0.1158 0.15 0.5] 점프
  (if (`self.CanPerformAction`)
    (if (not (`self.IsGuarding`))
      (switch `/Game/BluePrints/Character/EPlayerState` (`self.State_BP`)
        (:`NewEnumerator0`
          (`self.Jump`))))))

(event `Remote_Move_Triggered`
  (params (ActionValueX :type "Float (double-precision)") (ActionValueY :type "Float (double-precision)"))
  (bind (_returnvalue_roll _returnvalue_pitch _returnvalue_yaw) (`KismetMathLibrary.BreakRotator` (`self.GetControlRotation`)))
  ; 이동
  (if (`self.CanPerformAction`)
    (if (not (`self.IsGuarding`))
      (switch `/Game/BluePrints/Character/EPlayerState` (`self.State_BP`)
        (:`NewEnumerator0`
          (`self.AddMovementInput` (`KismetMathLibrary.GetRightVector` (`self.GetControlRotation`)) ActionValueX)
          (`self.AddMovementInput` (`KismetMathLibrary.GetForwardVector` (`KismetMathLibrary.MakeRotator` 0.0 0.0 _returnvalue_yaw)) ActionValueY))))))

(event `Remote_Move_Started`
  ; 이동
  ;[0.15 0.002204 0 0.5] 대쉬
  (if (<= (- (`KismetSystemLibrary.GetGameTimeInSeconds`) (`self.LastTapTime`)) 0.25)
    (set `self.IsDashing` true)
    (set `CharacterMovementComponent.MaxWalkSpeed` 800.0 (`self.CharacterMovement`))))

(event `Remote_Move_Completed`
  ;[0.15 0.002204 0 0.5] 대쉬
  (set `self.LastTapTime` (`KismetSystemLibrary.GetGameTimeInSeconds`))
  (set `self.IsDashing` false)
  (set `CharacterMovementComponent.MaxWalkSpeed` 400.0 (`self.CharacterMovement`)))

(event `Remote_Attack_Started`
  (bind _charactermovement (`self.CharacterMovement`))
  (bind _charactermovement_2 (`self.CharacterMovement`))
  (if (`self.CanPerformAction`)
    (if (`self.IsGuarding`)
      _
      (elif (`self.IsDashing`)
        ;[0.09308 0.15 0.005878 0.5] 대쉬 공격
        (set `self.IsDashing` false)
        (`Controller.SetIgnoreMoveInput` (`self.GetController`) true)
        (set `CharacterMovementComponent.GroundFriction` 0.0 _charactermovement_2)
        (set `CharacterMovementComponent.BrakingDecelerationWalking` 0.0 _charactermovement_2)
        (`self.PlayAnimMontage` (`self.DashAttack_M`))
        (`self.LaunchCharacter` (* (`self.GetActorForwardVector`) 900.0) true)
        (`KismetSystemLibrary.Delay` 0.8)
        (`Controller.SetIgnoreMoveInput` (`self.GetController`) false)
        (set `CharacterMovementComponent.GroundFriction` 8.0 _charactermovement)
        (set `CharacterMovementComponent.BrakingDecelerationWalking` 2048.0 _charactermovement)
        (set `CharacterMovementComponent.MaxWalkSpeed` 400.0 _charactermovement)
        (else
          ;[0 0.04439 0.15 0.5] 일반공격(펀치)
          (switch `/Game/BluePrints/Character/EPlayerState` (`self.State_BP`)
            (:`NewEnumerator0`
              (set `self.State_BP` "NewEnumerator1")
              (`self.PlayAnimMontage` "/Game/BluePrints/Character/Combat/AM_PunchCombo.AM_PunchCombo" 1.0 "None"))
            (:`NewEnumerator1`
              (switch `name` (`AnimInstance.Montage_GetCurrentSection` (`SkeletalMeshComponent.GetAnimInstance` (`self.Mesh`)) "/Game/BluePrints/Character/Combat/AM_PunchCombo.AM_PunchCombo")
                (:`Punch1`
                  (set `self.NextCombo` "Punch2"))
                (:`Punch2`
                  (set `self.NextCombo` "Punch3"))))))))))

(event `CustomEvent`
  ;[0 0.04439 0.15 0.5] 일반공격(펀치)
  (set `self.State_BP` "NewEnumerator0"))

(event `Remote_Guard_Started`
  (if (`self.ISCanMove`)
    (if (`self.CanPerformAction`)
      (set `self.IsGuarding` true))))

(event `Remote_Guard_Completed`
  (set `self.IsGuarding` false))

(fn `UserConstructionScript`)