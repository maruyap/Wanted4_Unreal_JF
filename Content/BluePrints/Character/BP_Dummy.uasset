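; BP_Dummy is a character that serves as a dummy target, printing any damage it receives.
; Its SendKnockback event launches it with the given velocity, overriding horizontal and vertical motion.
; After a short fixed delay it disables movement, then restores walking once the remaining stun duration has elapsed.
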(event `self.ReceiveAnyDamage`
  (params (Damage :type "Float (single-precision)") (DamageType :type "DamageType Object Reference") (InstigatedBy :type "Controller Object Reference") (DamageCauser :type "Actor Object Reference"))
  (`KismetSystemLibrary.PrintString` (`KismetStringLibrary.Conv_DoubleToString` Damage)))

(event `/Game/BluePrints/Character/BPI_Attackable.SendKnockback`
  (params (LaunchVelocity :type "Vector Structure") (StunDuration :type "Float (double-precision)") (IsHardSturn :type Boolean))
  (`self.LaunchCharacter` LaunchVelocity true true)
  (`KismetSystemLibrary.Delay` 0.3)
  (`CharacterMovementComponent.DisableMovement` (`self.CharacterMovement`))
  (`KismetSystemLibrary.Delay` (- StunDuration 0.3))
  (`CharacterMovementComponent.SetMovementMode` (`self.CharacterMovement`) "MOVE_Walking" 0))

(fn `UserConstructionScript`)