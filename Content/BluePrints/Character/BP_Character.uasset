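; Player character Blueprint that handles jumping, camera-relative movement and a double-tap dash through Enhanced Input.
; Jump and movement act only in the Locomotion state of StateBP, with movement following control rotation.
; Restarting move input shortly after releasing it raises max walk speed for a dash, regardless of state.
; Releasing move input timestamps the tap and restores normal speed.
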(event `EnhancedInput|/Game/BluePrints/Input/Actions/IA_Jump`
  (params (ActionValue :type Boolean) (ElapsedSeconds :type "Float (double-precision)") (TriggeredSeconds :type "Float (double-precision)") (InputAction :type "InputAction Object Reference" :default "/Game/BluePrints/Input/Actions/IA_Jump.IA_Jump"))
  ;[0.00526 0.1158 0.15 0.5] 점프
  (:`Started`
    (switch `/Game/BluePrints/Character/EPlayerState` (`self.State_BP`)
      (:`NewEnumerator0`
        (`self.Jump`)))))

(event `EnhancedInput|/Game/BluePrints/Input/Actions/IA_Move`
  (params (ActionValue :type "Vector2D Structure") (ElapsedSeconds :type "Float (double-precision)") (TriggeredSeconds :type "Float (double-precision)") (InputAction :type "InputAction Object Reference" :default "/Game/BluePrints/Input/Actions/IA_Move.IA_Move"))
  (bind (_returnvalue_roll _returnvalue_pitch _returnvalue_yaw) (`KismetMathLibrary.BreakRotator` (`self.GetControlRotation`)))
  ; 이동
  (:`Triggered`
    (switch `/Game/BluePrints/Character/EPlayerState` (`self.State_BP`)
      (:`NewEnumerator0`
        (`self.AddMovementInput` (`KismetMathLibrary.GetRightVector` (`self.GetControlRotation`)) ActionValue_X)
        (`self.AddMovementInput` (`KismetMathLibrary.GetForwardVector` (`KismetMathLibrary.MakeRotator` 0.0 0.0 _returnvalue_yaw)) ActionValue_Y))))
  (:`Started`
    ;[0.15 0.002204 0 0.5] 대쉬
    (if (<= (- (`KismetSystemLibrary.GetGameTimeInSeconds`) (`self.LastTapTime`)) 0.25)
      (set `self.IsDashing` true)
      (set `CharacterMovementComponent.MaxWalkSpeed` 1200.0 (`self.CharacterMovement`))))
  (:`Completed`
    (set `self.LastTapTime` (`KismetSystemLibrary.GetGameTimeInSeconds`))
    (set `self.IsDashing` false)
    (set `CharacterMovementComponent.MaxWalkSpeed` 600.0 (`self.CharacterMovement`))))

(fn `UserConstructionScript`)