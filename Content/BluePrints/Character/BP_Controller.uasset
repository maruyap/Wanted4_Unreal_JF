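; Player controller for local multiplayer that sets up input and a per-player health bar.
; On possess, it adds Enhanced Input mapping contexts by controller ID, with player 0 getting both game contexts and player 1 only IMC_Game2.
; A timer after BeginPlay creates WBP_HPBar on each local player's screen.
; It binds to the pawn's BP_HPController, repeats this on pawn changes, and sends HP ratio updates to the bar.
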(event `self.ReceivePossess`
  (params (PossessedPawn :type "Pawn Object Reference"))
  (switch `int` (`GameplayStatics.GetPlayerControllerID` self)
    (:`0`
      (`EnhancedInputSubsystemInterface.AddMappingContext` (subsystem `EnhancedInputLocalPlayerSubsystem`) "/Game/BluePrints/Input/IMC_Game.IMC_Game" 0 (struct))
      (`EnhancedInputSubsystemInterface.AddMappingContext` (subsystem `EnhancedInputLocalPlayerSubsystem`) "/Game/BluePrints/Input/IMC_Game2.IMC_Game2" 0 (struct)))
    (:`1`
      (`EnhancedInputSubsystemInterface.AddMappingContext` (subsystem `EnhancedInputLocalPlayerSubsystem`) "/Game/BluePrints/Input/IMC_Game2.IMC_Game2" 1 (struct)))))

(event `self.ReceiveBeginPlay`
  ; 각 플레이어 체력바 로직
  (`KismetSystemLibrary.K2_SetTimerDelegate` (delegate `delaytime`) 1.5))

(event `delaytime`
  ; 각 플레이어 체력바 로직
  (if (`self.IsLocalPlayerController`)
    (bind _returnvalue (`|CreateWidget` "/Game/BluePrints/UI/WBP_HPBar.WBP_HPBar_C" self))
    (bind _output_get (set `self.MyHPWidget` _returnvalue))
    (`UserWidget.AddToPlayerScreen` _output_get 0)
    (add `self.OnPossessedPawnChanged` (delegate `OnMyPawnChanged`))
    (`self.sethpbinding`)))

(event `OnMyPawnChanged` :!signature `self.OnPossessedPawnChanged`
  (params (OldPawn :type "Pawn Object Reference") (NewPawn :type "Pawn Object Reference"))
  ; 각 플레이어 체력바 로직
  (`self.sethpbinding`))

(event `sethpbinding`
  (bind _asbp_base_character (cast `/Game/BluePrints/Character/BP_BaseCharacter` (`self.K2_GetPawn`)))
  (bind _output_get (set `self.CurrentHPComponent` (`self.GetComponentByClass` _asbp_base_character "/Game/BluePrints/Components/BP_HPController.BP_HPController_C")))
  (add `/Game/BluePrints/Components/BP_HPController.OnHPChanged` _output_get (delegate `updateHUD`)))

(event `updateHUD`
  (params (HealthPower :type "Float (double-precision)") (MaxHealthPower :type "Float (double-precision)"))
  (`/Game/BluePrints/UI/WBP_HPBar.UpdateHpPercent` (`self.MyHPWidget`) (/ HealthPower MaxHealthPower)))

(fn `UserConstructionScript`)