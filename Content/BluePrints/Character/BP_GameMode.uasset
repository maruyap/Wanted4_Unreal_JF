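; Game mode that sets up a two-player local multiplayer session.
; BeginPlay creates a second local player, waits briefly, then replaces both default pawns with BP_BaseCharacter at the first PlayerStart found and BP_Player2 at the P2-tagged start, each possessed by its controller.
; Input-device hotplug handlers exist, but their binding is disconnected, alongside several unused spawn attempts.
; The ChoosePlayerStart override returns no start.
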(event `OnInputDeviceConnectionChange_Event`
  (params (NewConnectionState :type "EInputDeviceConnectionState Enum" :default "Invalid") (PlatformUserId :type "PlatformUserId Structure") (InputDeviceId :type "InputDeviceId Structure"))
  (if (!= (`KismetStringLibrary.Conv_StringToInt` (`KismetStringLibrary.Conv_InputDeviceIdToString` InputDeviceId)) 0)
    (switch `EInputDeviceConnectionState` NewConnectionState
      (:`Disconnected`
        (bind _returnvalue (`InputDeviceLibrary.GetPlayerControllerFromInputDevice` InputDeviceId))
        (`GameplayStatics.RemovePlayer` _returnvalue true))
      (:`Connected`
        (`GameplayStatics.CreatePlayer` -1)))))

(event `ConnectExistingDevices`
  (bind _outinputdevices (`InputDeviceLibrary.GetAllInputDevices`))
  (for (_ _array_index) _outinputdevices
    (if (!= _array_index 0)
      (`GameplayStatics.CreatePlayer` -1))))

(event `self.ReceiveBeginPlay`
  (`KismetSystemLibrary.ExecuteConsoleCommand` "set MaxLocalPlayers 2" (`GameplayStatics.GetPlayerControllerFromID` 0))
  (`GameplayStatics.CreatePlayer` 1)
  (`KismetSystemLibrary.Delay` 0.2)
  (`self.K2_DestroyActor` (`GameplayStatics.GetPlayerPawn` 0))
  (`self.K2_DestroyActor` (`GameplayStatics.GetPlayerPawn` 1))
  (`KismetSystemLibrary.PrintString` "2p delete ")
  (bind _outactors (`GameplayStatics.GetAllActorsOfClass` "/Script/Engine.PlayerStart"))
  (bind _returnvalue_location (`KismetMathLibrary.BreakTransform` (`self.GetTransform` (`|GetArrayItem` _outactors))))
  (bind _returnvalue (`|SpawnActorFromClass` "/Game/BluePrints/Character/BP_BaseCharacter.BP_BaseCharacter_C" (`KismetMathLibrary.MakeTransform` _returnvalue_location) "Undefined" "MultiplyWithRoot" null null))
  (`Controller.Possess` (`GameplayStatics.GetPlayerControllerFromID` 0) _returnvalue)
  (bind _outactors_2 (`GameplayStatics.GetAllActorsOfClassWithTag` "/Script/Engine.PlayerStart" "P2"))
  (bind _returnvalue_location_2 (`KismetMathLibrary.BreakTransform` (`self.GetTransform` (`|GetArrayItem` _outactors_2))))
  (bind _returnvalue_2 (`|SpawnActorFromClass` "/Game/BluePrints/Character/BP_Player2.BP_Player2_C" (`KismetMathLibrary.MakeTransform` _returnvalue_location_2) "Undefined" "MultiplyWithRoot" null null))
  (`Controller.Possess` (`GameplayStatics.GetPlayerControllerFromID` 1) _returnvalue_2))

(fn `ChoosePlayerStart`
  (params (Player :type "Controller Object Reference"))
  (returns (ReturnValue :type "Actor Object Reference"))
  (return null))

(fn `UserConstructionScript`)